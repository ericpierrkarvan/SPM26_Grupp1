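; BP_DoorLight_A is an indicator light that shows the on or off state of its InteractableReceiver, presumably for a door.
; The construction script starts the SpotLight in the off color.
; On BeginPlay it binds to the receiver's activation change, which switches the light color and swaps mesh materials.
; The material swap targets different slots: M_On goes to element 1, M_Off to element 0.
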(event Custom|OnActivationChanged_Event
  (params (Interactor :type Actor%20Object%20Reference) (IsOn :type Boolean))
  (if IsOn
    (Rendering|Material|SetMaterial (Variables|Default|GetMesh) 1 "/Game/Materials/M_On.M_On")
    (Rendering|Components|Light|SetLightColor (Variables|Default|GetSpotLight) (Variables|Default|GetOnColor) true)
    (else
      (Rendering|Material|SetMaterial (Variables|Default|GetMesh) 0 "/Game/Materials/M_Off.M_Off")
      (Rendering|Components|Light|SetLightColor (Variables|Default|GetSpotLight) (Variables|Default|GetOffColor) true))))

(event EventBeginPlay
  (EventDispatchers|AssignOnActivationChanged (Variables|Default|GetInteractableReceiver) (delegate Custom|OnActivationChanged_Event)))

(event Collision|EventActorBeginOverlap
  (params (OtherActor :type Actor%20Object%20Reference)))

(event EventTick
  (params (DeltaSeconds :type Float%20%28single-precision%29)))

(fn ConstructionScript
  (Rendering|Components|Light|SetLightColor (Variables|Default|GetSpotLight) (Variables|Default|GetOffColor) true))