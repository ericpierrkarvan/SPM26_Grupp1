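; Door interactable whose light material shows whether its receiver is activated.
; On BeginPlay it runs the parent logic, then binds to the ReceiverComponent's activation-changed event.
; Each change passes the on/off state to SetMaterials, which swaps a single mesh material slot (index 1) between the on and off light materials.
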(event Custom|OnActivationChanged_Event
  (params (Interactor :type Actor%20Object%20Reference) (IsOn :type Boolean))
  (CallFunction|SetMaterials IsOn))

(event EventBeginPlay
  (|CallParentFunction)
  (EventDispatchers|AssignOnActivationChanged (Variables|Default|GetReceiverComponent) (delegate Custom|OnActivationChanged_Event)))

(event Collision|EventActorBeginOverlap
  (params (OtherActor :type Actor%20Object%20Reference))
  (|CallParentFunction OtherActor) ; This node is disabled and will not be called.\nDrag off pins to build functionality.
)

(event EventTick
  (params (DeltaSeconds :type Float%20%28single-precision%29))
  (|CallParentFunction DeltaSeconds) ; This node is disabled and will not be called.\nDrag off pins to build functionality.
)

(fn ConstructionScript
  (|CallParentFunction))

(fn SetMaterials
  (params (IsOn :type Boolean))
  (if IsOn
    (Rendering|Material|SetMaterial (Variables|Character|GetMesh) 1 (Variables|Default|GetLightMatOn))
    (else
      (Rendering|Material|SetMaterial (Variables|Character|GetMesh) 1 (Variables|Default|GetLightMatOff)))))