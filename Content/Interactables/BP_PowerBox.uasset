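; BP_PowerBox is an interactable power box that shows its on/off state by swapping the mesh material.
; OnOffState applies the on or off material, first from the Interactable's StartsOn value at BeginPlay, then from each OnInteract event's IsOn value.
; Each interaction also plays an electric sound event at the actor's location.
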(event OnInteract(Interactable)
  (params (Interactor :type Actor%20Object%20Reference) (IsOn :type Boolean))
  (CallFunction|OnOffState IsOn)
  (Class|FMODBlueprintStatics|PlayEventatLocation "/Game/FMOD/Events/MISC/InteractElectric.InteractElectric" (Math|Conversions|ToTransform(Vector) (Transformation|GetActorLocation))))

(event EventBeginPlay
  ;[0.15 0.15 0.15 0.5] Set lamp color
  (CallFunction|OnOffState (Variables|/Script/SPM26_Grupp1.InteractableComponent|GetbStartsOn (Variables|Default|GetInteractable))))

(event Collision|EventActorBeginOverlap
  (params (OtherActor :type Actor%20Object%20Reference)))

(event EventTick
  (params (DeltaSeconds :type Float%20%28single-precision%29)))

(fn ConstructionScript)

(fn OnOffState
  (params (NewState :type Boolean))
  (if NewState
    (Rendering|Material|SetMaterial (Variables|Debug|GetStaticMeshComponent) 0 "/Game/Materials/M_On.M_On")
    (else
      (Rendering|Material|SetMaterial (Variables|Debug|GetStaticMeshComponent) 0 "/Game/Materials/M_Off.M_Off"))))