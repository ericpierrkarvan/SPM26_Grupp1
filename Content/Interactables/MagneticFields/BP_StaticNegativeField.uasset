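; BP_StaticNegativeField is a switchable negative magnetic field that handles sound feedback for actors it affects.
; Its InteractableReceiver activates or disables the field when its on/off state changes.
; Inherited pull, repulsion and force-end events play or stop sounds through each affected actor's MagneticComponent, and EndPlay silences every actor still in the field.
; BeginPlay also adds an auto-destroying FMOD audio component.
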(event OnActivationChanged(InteractableReceiver)
  (params (Interactor :type Actor%20Object%20Reference) (IsOn :type Boolean))
  ;[0.15 0.15 0.15 0.5] Switch on/off field
  (if IsOn
    (Class|MagneticFieldCylinder|Activate)
    (else
      (Class|MagneticFieldCylinder|Disable))))

(event Collision|EventActorBeginOverlap
  (params (OtherActor :type Actor%20Object%20Reference))
  (|CallParentFunction OtherActor) ; This node is disabled and will not be called.\nDrag off pins to build functionality.
)

(event EventEndPlay
  (params (EndPlayReason :type EEndPlayReason%20Enum :default "Destroyed"))
  (for _array_element (Variables|Default|GetActorsInField)
    (if (Utilities|IsValid _array_element)
      (Class|MagneticComponent|StopMagneticSounds (Actor|GetComponentbyClass _array_element "/Script/SPM26_Grupp1.MagneticComponent")))))

(event EventBeginPlay
  (AddComponent|AddFMODAudioComponent false)
  (Variables|Default|SetbAutoDestroyWhenFinished true))

(event EventTick
  (params (DeltaSeconds :type Float%20%28single-precision%29))
  (|CallParentFunction DeltaSeconds) ; This node is disabled and will not be called.\nDrag off pins to build functionality.
)

(event EventOnMagneticPullBP
  (params (Actor :type Actor%20Object%20Reference))
  (bind _returnvalue (Actor|GetComponentbyClass Actor "/Script/SPM26_Grupp1.MagneticComponent"))
  ;[0.15 0.15 0.15 0.5] Play Pull Sound
  (if (Utilities|IsValid Actor)
    (Utilities|IsValid _returnvalue
      (:Is%20Valid
        (Class|MagneticComponent|PlayPullSound _returnvalue)))))

(event EventOnMagneticRepulsionBP
  (params (Actor :type Actor%20Object%20Reference))
  (bind _returnvalue (Actor|GetComponentbyClass Actor "/Script/SPM26_Grupp1.MagneticComponent"))
  ;[0.15 0.15 0.15 0.5] Play Repel Sound
  (if (Utilities|IsValid Actor)
    (Utilities|IsValid _returnvalue
      (:Is%20Valid
        (Class|MagneticComponent|PlayRepelSound _returnvalue)))))

(event EventOnMagneticForceEndBP
  (params (Actor :type Actor%20Object%20Reference))
  (bind _returnvalue (Actor|GetComponentbyClass Actor "/Script/SPM26_Grupp1.MagneticComponent"))
  (if (Utilities|IsValid Actor)
    (Utilities|IsValid _returnvalue
      (:Is%20Valid
        (Class|MagneticComponent|StopMagneticSounds _returnvalue)))))

(fn ConstructionScript
  (|CallParentFunction))