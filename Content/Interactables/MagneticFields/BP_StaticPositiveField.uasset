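; BP_StaticPositiveField is an interactable magnetic field actor, named as a static positive field, that can be switched on and off.
; It responds to activation changes from its InteractableReceiver by calling Activate or Disable.
; It defines no field behavior of its own in these graphs, and its BeginPlay and construction script only call the parent.
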(event OnActivationChanged(InteractableReceiver)
  (params (Interactor :type Actor%20Object%20Reference) (IsOn :type Boolean))
  ;[0.15 0.15 0.15 0.5] Switch on/off field
  (if IsOn
    (Class|MagneticFieldCylinder|Activate)
    (else
      (Class|MagneticFieldCylinder|Disable))))

(event EventBeginPlay
  (|CallParentFunction))

(event Collision|EventActorBeginOverlap
  (params (OtherActor :type Actor%20Object%20Reference))
  (|CallParentFunction OtherActor) ; This node is disabled and will not be called.\nDrag off pins to build functionality.
)

(event EventTick
  (params (DeltaSeconds :type Float%20%28single-precision%29))
  (|CallParentFunction DeltaSeconds) ; This node is disabled and will not be called.\nDrag off pins to build functionality.
)

(fn ConstructionScript
  (|CallParentFunction))