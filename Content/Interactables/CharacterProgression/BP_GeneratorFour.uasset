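; BP_GeneratorFour is a scannable generator interactable, filed under character progression, that starts with actor collision disabled and responds to activation.
; It binds to its InteractableReceiver's activation-changed event on BeginPlay.
; Each change sets mesh gravity to the activation state, enables collision and clears the ShouldRotate flag, whether switched on or off.
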(event Custom|OnActivationChanged_Event
  (params (Interactor :type Actor%20Object%20Reference) (IsOn :type Boolean))
  (Physics|SetEnableGravity (Variables|Default|GetMeshComponent) IsOn)
  (Collision|SetActorEnableCollision true)
  (Variables|Default|SetShouldRotate false))

(event EventBeginPlay
  (|CallParentFunction)
  (Collision|SetActorEnableCollision false)
  (EventDispatchers|AssignOnActivationChanged (Variables|Default|GetInteractableReceiver) (delegate Custom|OnActivationChanged_Event)))

(event Collision|EventActorBeginOverlap
  (params (OtherActor :type Actor%20Object%20Reference))
  (|CallParentFunction OtherActor) ; This node is disabled and will not be called.\nDrag off pins to build functionality.
)

(event EventTick
  (params (DeltaSeconds :type Float%20%28single-precision%29))
  (|CallParentFunction DeltaSeconds) ; This node is disabled and will not be called.\nDrag off pins to build functionality.
)

(fn ConstructionScript
  (|CallParentFunction))

(fn IsScannable
  (return true))