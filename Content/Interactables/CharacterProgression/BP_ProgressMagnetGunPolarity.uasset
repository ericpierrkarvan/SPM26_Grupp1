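; A character progression pickup, by its name the magnet gun polarity switch unlock.
; On BeginPlay it runs the parent logic, then looks up the MagneticGunPolaritySwitch row in the ProgressionPromptText data table.
; The row's Title becomes the pickup component's prompt text.
; All other behavior comes from the parent class; Tick and the construction script only call their parents.
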(event EventBeginPlay
  (|CallParentFunction)
  (bind _returnvalue (Utilities|GetDataTableRow "/Game/UI/ProgressionPrompt/ProgressionPromptText.ProgressionPromptText" "MagneticGunPolaritySwitch")
    (:then
      (Variables|/Script/SPM26_Grupp1.PickupComponent|SetPickupPromptText (Variables|Default|GetPickupComponent) (Utilities|Text|ToText(String) (.title _returnvalue))))))

(event Collision|EventActorBeginOverlap
  (params (OtherActor :type Actor%20Object%20Reference))
  (|CallParentFunction OtherActor) ; This node is disabled and will not be called.\nDrag off pins to build functionality.
)

(event EventTick
  (params (DeltaSeconds :type Float%20%28single-precision%29))
  (|CallParentFunction DeltaSeconds))

(fn ConstructionScript
  (|CallParentFunction))