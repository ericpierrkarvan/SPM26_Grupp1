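; Base Blueprint for a character progression pickup that continuously rotates in the world.
; Each Tick orbits the actor's location around its RotatePoint component on the vertical axis and adds a small rotation to the actor.
; The step is a fixed angle per frame, not scaled by DeltaSeconds, so speed depends on frame rate.
; No collection or progression logic lives in these graphs.
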(event EventBeginPlay
  (|CallParentFunction) ; This node is disabled and will not be called.\nDrag off pins to build functionality.
)

(event Collision|EventActorBeginOverlap
  (params (OtherActor :type Actor%20Object%20Reference))
  (|CallParentFunction OtherActor) ; This node is disabled and will not be called.\nDrag off pins to build functionality.
)

(event EventTick
  (params (DeltaSeconds :type Float%20%28single-precision%29))
  (|CallParentFunction DeltaSeconds)
  (Transformation|SetActorLocationAndRotation (+ (Transformation|GetWorldLocation (Variables|Default|GetRotatePoint)) (Math|Vector|RotateVectorAroundAxis (- (Transformation|GetActorLocation) (Transformation|GetWorldLocation (Variables|Default|GetRotatePoint))) 1.0 "0.000000,0.000000,1.000000")) (Math|Rotator|CombineRotators (Transformation|GetActorRotation) "0.000000,1.000000,0.000000")))

(fn ConstructionScript
  (|CallParentFunction))