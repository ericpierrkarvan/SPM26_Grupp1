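; BP_PowerSwitch is an interactable switch actor whose mesh shows its on or off state.
; The Interactable component's OnInteract event passes the new state to Setstate and plays the HumanScan sound event at the actor's location.
; BeginPlay applies the component's StartsOn value through the same function.
; Setstate swaps two mesh material slots between powered and unpowered emissive and screen materials.
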(event OnInteract(Interactable)
  (params (Interactor :type Actor%20Object%20Reference) (IsOn :type Boolean))
  (CallFunction|Setstate IsOn)
  (Class|FMODBlueprintStatics|PlayEventatLocation "/Game/FMOD/Events/MISC/HumanScan.HumanScan" (Math|Conversions|ToTransform(Vector) (Transformation|GetActorLocation))))

(event EventBeginPlay
  (CallFunction|Setstate (Variables|/Script/SPM26_Grupp1.InteractableComponent|GetbStartsOn (Variables|Default|GetInteractable))))

(event Collision|EventActorBeginOverlap
  (params (OtherActor :type Actor%20Object%20Reference)))

(event EventTick
  (params (DeltaSeconds :type Float%20%28single-precision%29)))

(fn ConstructionScript)

(fn Setstate
  (params (Condition :type Boolean))
  (if Condition
    (Rendering|Material|SetMaterial (Variables|Debug|GetStaticMeshComponent) 1 "/Engine/ArtTools/RenderToTexture/Materials/Debug/M_Emissive_Color_0-0-127.M_Emissive_Color_0-0-127")
    (Rendering|Material|SetMaterial (Variables|Debug|GetStaticMeshComponent) 2 "/Game/Materials/M_CRT_Scanlines.M_CRT_Scanlines")
    (else
      (Rendering|Material|SetMaterial (Variables|Debug|GetStaticMeshComponent) 1 "/Engine/ArtTools/RenderToTexture/Materials/Debug/M_Emissive_Color_127-127-0.M_Emissive_Color_127-127-0")
      (Rendering|Material|SetMaterial (Variables|Debug|GetStaticMeshComponent) 2 "/Game/Materials/M_BoxScreen.M_BoxScreen"))))