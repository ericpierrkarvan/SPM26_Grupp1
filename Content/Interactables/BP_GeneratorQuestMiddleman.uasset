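; Generator quest middleman that links two interactable receivers, A and B, to the quest text in the UI.
; On BeginPlay it binds each receiver's activation-changed event to its own handler.
; Each handler toggles its active flag through a FlipFlop, ignoring the IsOn value, so state follows the count of changes.
; It then broadcasts show-quest-text through the UI subsystem with the OR of both flags.
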(event Custom|OnActivationChanged_A
  (params (Interactor :type Actor%20Object%20Reference) (IsOn :type Boolean))
  (Utilities|FlowControl|FlipFlop
    (:A
      (Variables|Default|SetAActive true))
    (:B
      (Variables|Default|SetAActive false)))
  (Class|UISubSystem|BroadcastShowQuestText (Subsystems|GetUISubSystem) (or (Variables|Default|GetBActive) (Variables|Default|GetAActive))))

(event Custom|OnActivationChanged_B
  (params (Interactor :type Actor%20Object%20Reference) (IsOn :type Boolean))
  (Utilities|FlowControl|FlipFlop
    (:A
      (Variables|Default|SetBActive true))
    (:B
      (Variables|Default|SetBActive false)))
  (Class|UISubSystem|BroadcastShowQuestText (Subsystems|GetUISubSystem) (or (Variables|Default|GetBActive) (Variables|Default|GetAActive))))

(event EventBeginPlay
  (EventDispatchers|AssignOnActivationChanged (Variables|Default|GetInteractableReceiver_A) (delegate Custom|OnActivationChanged_A))
  (EventDispatchers|AssignOnActivationChanged (Variables|Default|GetInteractableReceiver_B) (delegate Custom|OnActivationChanged_B)))

(fn ConstructionScript)