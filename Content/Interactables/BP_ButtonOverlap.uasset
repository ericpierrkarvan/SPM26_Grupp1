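; A one-shot target button that triggers a linked Interactable when a pawn, dynamic object or physics body overlaps its detection cylinder.
; On first overlap the target mesh detaches, switches to its "on" material and falls under physics with a sound, while detection shuts off.
; Hard hits on the fallen mesh play impact sounds, rate-limited by a timer counted down on Tick.
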(event Custom|OnComponentBeginOverlap_Event
  (params (OverlappedComponent :type Primitive%20Component%20Object%20Reference) (OtherActor :type Actor%20Object%20Reference) (OtherComp :type Primitive%20Component%20Object%20Reference) (OtherBodyIndex :type Integer) (bFromSweep :type Boolean) (SweepResult :type Hit%20Result%20Structure%20%28by%20ref%29))
  (bind _targetmesh (Variables|Default|GetTargetMesh))
  ;[0.15 0.15 0.15 0.5] Target startsto fall down
  (Utilities|FlowControl|DoOnce false
    (:Completed
      ;;[0.15 0.02122 0.1095 0.502] Detach Sound
      (Class|FMODBlueprintStatics|PlayEventAttached 0 0 "None" "0, 0, 0" "KeepRelativeOffset")
      (Transformation|DetachFromComponent (Variables|Default|GetTargetMesh) "KeepWorld" "KeepWorld" "KeepWorld" true)
      (Collision|SetCollisionResponsetoAllChannels (Variables|Default|GetCylinderCollisionDetection) "ECR_Ignore")
      (Physics|SetSimulatePhysics _targetmesh true)
      (Class|PrimitiveComponent|SetNotifyRigidBodyCollision _targetmesh true)
      (Rendering|Material|SetMaterial _targetmesh 0 "/Game/Materials/M_On.M_On")
      (Components|Activation|Deactivate (Variables|Default|GetCylinderCollisionDetection))
      (Class|InteractableComponent|Interact (Variables|Default|GetInteractable))
      (Collision|BindEventtoOnComponentHit (Variables|Default|GetTargetMesh) (delegate Custom|OnTargetCollision))
      (Variables|Default|SettargetFellDown true))))

(event Custom|OnTargetCollision
  (params (HitComponent :type Primitive%20Component%20Object%20Reference) (OtherActor :type Actor%20Object%20Reference) (OtherComp :type Primitive%20Component%20Object%20Reference) (NormalImpulse :type Vector) (Hit :type Hit%20Result%20Structure%20%28by%20ref%29))
  (if (and (> (Math|Vector|VectorLength NormalImpulse) 1e+05) (<= (Variables|Default|GetSoundTimer) 0.0))
    ;[0.15 0.02122 0.1095 0.502] Collide sound - when the target falls down etc
    (Class|FMODBlueprintStatics|PlayEventAttached 0 (Variables|Default|GetTargetMesh) "None" "0, 0, 0" "KeepRelativeOffset")
    ;[0.15 0.15 0.15 0.5] how often can we play impact sound
    (Variables|Default|SetSoundTimer 0.3)))

(event EventBeginPlay
  (bind _cylindercollisiondetection (Variables|Default|GetCylinderCollisionDetection))
  ;[0.15 0.15 0.15 0.5] BeginPlay
  (Collision|SetCollisionEnabled _cylindercollisiondetection "QueryOnly")
  (Collision|SetCollisionResponsetoAllChannels _cylindercollisiondetection "ECR_Ignore")
  (Collision|SetCollisionResponsetoChannel _cylindercollisiondetection "ECC_Pawn" "ECR_Overlap")
  (Collision|SetCollisionResponsetoChannel _cylindercollisiondetection "ECC_WorldDynamic" "ECR_Overlap")
  (Collision|SetCollisionResponsetoChannel _cylindercollisiondetection "ECC_PhysicsBody" "ECR_Overlap")
  (Collision|AssignOnComponentBeginOverlap (Variables|Default|GetCylinderCollisionDetection) (delegate Custom|OnComponentBeginOverlap_Event)))

(event EventTick
  (params (DeltaSeconds :type Float%20%28single-precision%29))
  ;[0.15 0.15 0.15 0.5] Tick
  (if (Variables|Default|GettargetFellDown)
    (Variables|Default|SetSoundTimer (- (Variables|Default|GetSoundTimer) DeltaSeconds))))

(fn ConstructionScript)