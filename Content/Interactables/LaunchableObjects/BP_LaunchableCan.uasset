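; Launchable can interactable that plays an impact sound when the player touches it or it takes a strong hit.
; Hit handling binds after a short random delay from BeginPlay, and a cooldown timer limits repeat sounds.
; Tick counts the cooldown down, with PickupComponent enabling tick on pickup and Respawn disabling it on respawn.
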(event Custom|OnPickedUpDelegate_Event
  (params (ByActor :type Actor%20Object%20Reference))
  (Actor|Tick|SetActorTickEnabled true))

(event Custom|OnActorHit_Event
  (params (SelfActor :type Actor%20Object%20Reference) (OtherActor :type Actor%20Object%20Reference) (NormalImpulse :type Vector) (Hit :type Hit%20Result%20Structure%20%28by%20ref%29))
  (if (and (or (Actor|ActorHasTag OtherActor "Player") (> (Math|Vector|VectorLength NormalImpulse) 1e+05)) (== (Variables|Default|GetSoundImpactTimer) 0.0))
    (Class|FMODBlueprintStatics|PlayEventatLocation (Variables|Default|GetImpactSound) (Math|Conversions|ToTransform(Vector) (Transformation|GetActorLocation)))
    (Variables|Default|SetSoundImpactTimer (Variables|Default|GetSoundImpactCooldown))))

(event Custom|OnRespawned_Event
  (Actor|Tick|SetActorTickEnabled false))

(event EventBeginPlay
  (EventDispatchers|AssignOnPickedUpDelegate (Variables|Default|GetPickupComponent) (delegate Custom|OnPickedUpDelegate_Event))
  (EventDispatchers|AssignOnRespawned (Variables|Default|GetRespawn) (delegate Custom|OnRespawned_Event))
  (Utilities|FlowControl|Delay (Math|Random|RandomFloatinRange 1.5 2.0))
  (Collision|AssignOnActorHit (delegate Custom|OnActorHit_Event)))

(event Collision|EventActorBeginOverlap
  (params (OtherActor :type Actor%20Object%20Reference)))

(event EventTick
  (params (DeltaSeconds :type Float%20%28single-precision%29))
  (if (> (Variables|Default|GetSoundImpactTimer) 0.0)
    (Variables|Default|SetSoundImpactTimer (Math|Float|Clamp(Float) (- (Variables|Default|GetSoundImpactTimer) DeltaSeconds) 0.0 (Variables|Default|GetSoundImpactCooldown)))))

(fn ConstructionScript)