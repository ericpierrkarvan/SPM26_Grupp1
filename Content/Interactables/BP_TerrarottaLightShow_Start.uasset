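; Interactable Blueprint that kicks off the Terrarotta light show when its receiver switches on.
; On BeginPlay it binds to InteractableReceiverA's activation change and caches its own location for audio.
; On activation it plays a start sound, waits briefly, then force-activates Interactable1 and plays a second sound.
; Deactivation is ignored, and the sounds reuse door and menu events.
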(event Custom|OnActivationChanged_Event
  (params (Interactor :type Actor%20Object%20Reference) (IsOn :type Boolean))
  (if IsOn
    ;[0.15 0.15 0.15 0.5] Sound: lightshow start. Cave crumblesound?
    (Class|FMODBlueprintStatics|PlayEventatLocation "/Game/FMOD/Events/MISC/BigDoorOpenStart.BigDoorOpenStart" (Variables|Default|GetSoundLoc))
    (Utilities|FlowControl|Delay 1.8)
    (Class|InteractableComponent|ForceInteract (Variables|Default|GetInteractable1) true)
    (Class|FMODBlueprintStatics|PlayEventatLocation "/Game/FMOD/Events/INTERFACE/CloseMenu.CloseMenu" (Variables|Default|GetSoundLoc))))

(event EventBeginPlay
  (EventDispatchers|AssignOnActivationChanged (Variables|Default|GetInteractableReceiver_A) (delegate Custom|OnActivationChanged_Event))
  (Variables|Default|SetSoundLoc (Math|Conversions|ToTransform(Vector) (Transformation|GetActorLocation))))

(fn ConstructionScript)