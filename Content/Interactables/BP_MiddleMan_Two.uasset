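; BP_MiddleMan_Two is an interactable relay that combines two receivers into one AND-gated output.
; On BeginPlay it binds to the activation changes of InteractableReceiverA and InteractableReceiverB, caching each state.
; Either change force-sets InteractableA to active only when both inputs are on, passing the interactor through.
; Changes on A also call a plain Interact on InteractableA before the forced state, unlike changes on B.
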(event Custom|OnActivationChanged_A
  (params (Interactor :type Actor%20Object%20Reference) (IsOn :type Boolean))
  (Variables|Default|SetAActive IsOn)
  (Class|InteractableComponent|Interact (Variables|Default|GetInteractable_A) Interactor)
  (Class|InteractableComponent|ForceInteract (Variables|Default|GetInteractable_A) (and (Variables|Default|GetBActive) (Variables|Default|GetAActive)) Interactor))

(event Custom|OnActivationChanged_B
  (params (Interactor :type Actor%20Object%20Reference) (IsOn :type Boolean))
  (Variables|Default|SetBActive IsOn)
  (Class|InteractableComponent|ForceInteract (Variables|Default|GetInteractable_A) (and (Variables|Default|GetBActive) (Variables|Default|GetAActive)) Interactor))

(event EventBeginPlay
  (EventDispatchers|AssignOnActivationChanged (Variables|Default|GetInteractableReceiver_A) (delegate Custom|OnActivationChanged_A))
  (EventDispatchers|AssignOnActivationChanged (Variables|Default|GetInteractableReceiver_B) (delegate Custom|OnActivationChanged_B)))

(fn ConstructionScript)