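; Chain-link interactable for the Terrarotta light show that passes an activation on after a delay.
; On BeginPlay it binds to InteractableReceiverA's activation change and caches its own location for audio.
; When switched on, it waits LightDelay, force-activates Interactable1 and plays the activation sound event at that location.
; Switch-off signals are ignored.
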(event Custom|OnActivationChanged_Event
  (params (Interactor :type Actor%20Object%20Reference) (IsOn :type Boolean))
  (if IsOn
    (Utilities|FlowControl|Delay (Variables|Default|GetLightDelay))
    (Class|InteractableComponent|ForceInteract (Variables|Default|GetInteractable1) true)
    ;[0.15 0.15 0.15 0.5] Lights
    (Class|FMODBlueprintStatics|PlayEventatLocation (Variables|Default|GetActivationSound) (Variables|Default|GetSoundLoc))))

(event EventBeginPlay
  (EventDispatchers|AssignOnActivationChanged (Variables|Default|GetInteractableReceiver_A) (delegate Custom|OnActivationChanged_Event))
  (Variables|Default|SetSoundLoc (Math|Conversions|ToTransform(Vector) (Transformation|GetActorLocation))))

(fn ConstructionScript)