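; Fleeing alien NPC variant that carries a floating item and releases it when pulled by telekinesis.
; Fleeing and patrolling events stop the current audio and attach a chase or idle sound event to the mesh.
; On BeginPlay it binds to the Telekinesis state change; entering Sucking launches the valid FloatingItem and plays a robot launch sound at the alien's location.
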(event Custom|OnTelekinesisStateChanged_Event
  (params (NewState :type ETelekinesisState%20Enum :default "WaitingForKinetic"))
  (bind _floatingitem (Variables|Default|GetFloatingItem))
  (switch Utilities|FlowControl|Switch|SwitchonETelekinesisState NewState
    (:Sucking
      (Utilities|IsValid _floatingitem
        (:Is%20Valid
          (Class|FloatingItemComponent|LaunchItem _floatingitem)
          (Class|FMODBlueprintStatics|PlayEventatLocation "/Game/FMOD/Events/PLAYER/RobotLaunch.RobotLaunch" (Math|Conversions|ToTransform(Vector) (Transformation|GetActorLocation))))))))

(event EventBeginPlay
  (EventDispatchers|AssignOnTelekinesisStateChanged (Variables|Default|GetTelekinesis) (delegate Custom|OnTelekinesisStateChanged_Event)))

(event Collision|EventActorBeginOverlap
  (params (OtherActor :type Actor%20Object%20Reference)))

(event EventTick
  (params (DeltaSeconds :type Float%20%28single-precision%29)))

(event EventIsPatrollingBP
  (Class|FMODAudioComponent|Stop (Variables|Default|GetCurrentAudio))
  (bind _returnvalue (Class|FMODBlueprintStatics|PlayEventAttached "/Game/FMOD/Events/MISC/NPCidle.NPCidle" (Variables|Character|GetMesh) "None" "0, 0, 0" "KeepRelativeOffset"))
  (Variables|Default|SetCurrentAudio _returnvalue))

(event EventIsFleeingBP
  (Class|FMODAudioComponent|Stop (Variables|Default|GetCurrentAudio))
  (bind _returnvalue (Class|FMODBlueprintStatics|PlayEventAttached "/Game/FMOD/Events/MISC/NPCchase.NPCchase" (Variables|Character|GetMesh) "None" "0, 0, 0" "KeepRelativeOffset"))
  (Variables|Default|SetCurrentAudio _returnvalue))

(fn ConstructionScript)