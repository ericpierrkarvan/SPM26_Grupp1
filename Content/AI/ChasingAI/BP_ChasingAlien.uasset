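; Chasing alien AI character Blueprint that adds sound feedback to behavior state changes.
; Chase and patrol events stop the stored audio, then play the chase or idle audio event attached to the mesh and store it as the current one.
; Push-back plays a knock sound on the mesh without interrupting that loop reference, while the investigating event is left empty.
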(event EventBeginPlay)

(event Collision|EventActorBeginOverlap
  (params (OtherActor :type Actor%20Object%20Reference)))

(event EventTick
  (params (DeltaSeconds :type Float%20%28single-precision%29)))

(event EventAlienPushBackBP
  (Class|FMODBlueprintStatics|PlayEventAttached "/Game/FMOD/Events/MISC/NPCknock.NPCknock" (Variables|Character|GetMesh) "None" "0, 0, 0" "KeepRelativeOffset"))

(event EventIsChasingBP
  (Class|FMODAudioComponent|Stop (Variables|Default|GetCurrentAudio))
  (bind _returnvalue (Class|FMODBlueprintStatics|PlayEventAttached "/Game/FMOD/Events/MISC/NPCchase.NPCchase" (Variables|Character|GetMesh) "None" "0, 0, 0" "KeepRelativeOffset"))
  (Variables|Default|SetCurrentAudio _returnvalue))

(event EventIsPatrollingBP
  (Class|FMODAudioComponent|Stop (Variables|Default|GetCurrentAudio))
  (bind _returnvalue (Class|FMODBlueprintStatics|PlayEventAttached "/Game/FMOD/Events/MISC/NPCidle.NPCidle" (Variables|Character|GetMesh) "None" "0, 0, 0" "KeepRelativeOffset"))
  (Variables|Default|SetCurrentAudio _returnvalue))

(event EventIsInvestigatingBP)

(fn ConstructionScript)