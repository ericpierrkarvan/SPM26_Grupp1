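; Ship weapon doors actor that opens a left and right door when its interactable receiver is activated.
; It binds to the receiver's activation change on BeginPlay and plays a one-shot animation on each door.
; A HaveOpened flag makes opening one-way, so deactivation or repeat activations never close or replay the doors.
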(event Custom|OnActivationChanged_Event
  (params (Interactor :type Actor%20Object%20Reference) (IsOn :type Boolean))
  (if (and IsOn (not (Variables|Default|GethaveOpened)))
    (Components|Animation|PlayAnimation (Variables|Default|GetLeftDoor) "/Game/Animations/WeaponDoors/AS_WeaponDoor_L.AS_WeaponDoor_L" false)
    (Components|Animation|PlayAnimation (Variables|Default|GetRightDoor) "/Game/Animations/WeaponDoors/AS_WeaponDoor_R.AS_WeaponDoor_R" false)
    ;[0.15 0.15 0.15 0.5] cant close the doors again once opened
    (Variables|Default|SethaveOpened true)))

(event EventBeginPlay
  (EventDispatchers|AssignOnActivationChanged (Variables|Default|GetInteractableReceiver) (delegate Custom|OnActivationChanged_Event)))

(event Collision|EventActorBeginOverlap
  (params (OtherActor :type Actor%20Object%20Reference)))

(event EventTick
  (params (DeltaSeconds :type Float%20%28single-precision%29)))

(fn ConstructionScript)