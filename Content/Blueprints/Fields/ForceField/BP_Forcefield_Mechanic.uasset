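; Forcefield actor Blueprint that supplies FMOD audio for the forcefield mechanic.
; BeginPlay starts an attached static sound, with the parent BeginPlay call disabled.
; Pass-through events start and stop an attached sound via a stored component reference, while push-back plays a one-shot at the actor's location.
; An author note flags the pass-through pair as broken by double overlap events.
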(event EventBeginPlay
  (Class|FMODBlueprintStatics|PlayEventAttached "/Game/FMOD/Events/MISC/ForceFieldStatic.ForceFieldStatic" (Variables|Transformation|GetRootComponent) "None" "0, 0, 0" "KeepRelativeOffset"))

(event Collision|EventActorBeginOverlap
  (params (OtherActor :type Actor%20Object%20Reference)))

(event EventTick
  (params (DeltaSeconds :type Float%20%28single-precision%29)))

(event EventPushedBackBP
  (Class|FMODBlueprintStatics|PlayEventatLocation "/Game/FMOD/Events/MISC/ForceFieldPush.ForceFieldPush" (Math|Conversions|ToTransform(Vector) (Transformation|GetActorLocation))))

(event EventStopPassingThroughBP
  ;[0.15 0.15 0.15 0.5] PassingThrough + StopPassingThrough // BRICKED BY DOUBLE OVERLAP EVENTS
  (Utilities|IsValid (stale EventPassingThroughBP _output_get)
    (:Is%20Valid
      (Class|FMODAudioComponent|Stop (stale EventPassingThroughBP _output_get))
      (Variables|Default|SetFMODAudio 0))))

(event EventPassingThroughBP
  ;[0.15 0.15 0.15 0.5] PassingThrough + StopPassingThrough // BRICKED BY DOUBLE OVERLAP EVENTS
  (bind _returnvalue (Class|FMODBlueprintStatics|PlayEventAttached "/Game/FMOD/Events/MISC/ForceFieldPass.ForceFieldPass" (Variables|Transformation|GetRootComponent) "None" "0, 0, 0" "KeepRelativeOffset"))
  (bind _output_get (Variables|Default|SetFMODAudio _returnvalue)))

(fn ConstructionScript
  (|CallParentFunction))