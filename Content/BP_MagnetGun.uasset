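; BP_MagnetGun is the magnet gun Blueprint, and its graph handles only aim-down-sights and firing audio through FMOD-style events.
; OnShoot plays the fire event at the actor's location.
; OnADS creates the aim event there with auto-play off, never starting it, and stops ADSAudioComponent when aiming ends.
; Component SetEvent and Play calls remain unconnected, and the construction script is empty.
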(event EventOnADS
  (params (bIsADS :type Boolean))
  (if bIsADS
    (Class|FMODBlueprintStatics|PlayEventatLocation "/Game/FMOD/Events/MISC/MagnetGunADS.MagnetGunADS" (Math|Conversions|ToTransform(Vector) (Transformation|GetActorLocation)) false)
    (else
      (Class|FMODAudioComponent|Stop (Variables|Default|GetADSAudioComponent)))))

(event EventOnShoot
  (Class|FMODBlueprintStatics|PlayEventatLocation "/Game/FMOD/Events/MISC/MagnetGunFire.MagnetGunFire" (Math|Conversions|ToTransform(Vector) (Transformation|GetActorLocation))))

(fn ConstructionScript)