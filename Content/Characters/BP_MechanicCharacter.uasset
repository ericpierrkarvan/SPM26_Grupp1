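; Mechanic character Blueprint that supplies audio and visual feedback for magnetic polarity switches and double jumps.
; A switch to Positive adds an FMOD audio component, while Negative plays the existing polarity switch audio component.
; The movement component's double-jump event spawns a Niagara effect at the actor and adds FMOD audio.
; BeginPlay caches the first BP_NewMagneticFieldCylinder in the level, though these graphs never use it.
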(event DoubleJumpEvent(CharacterMovement)
  (params (JumpZVelocity :type Float%20%28single-precision%29))
  (Niagara|SpawnSystematLocation "/Game/ParticleSystems/CharacterSystems/NS_DoubleJump.NS_DoubleJump" (Transformation|GetActorLocation))
  (AddComponent|AddFMODAudioComponent false))

(event EventOnSwitchPolarity
  (params (NewPolarity :type EPolarity%20Enum :default "Positive"))
  (switch Utilities|FlowControl|Switch|SwitchonEPolarity NewPolarity
    (:Positive
      (AddComponent|AddFMODAudioComponent false))
    (:Negative
      (Class|FMODAudioComponent|Play (Variables|Default|GetPolaritySwitchAudioComp)))))

(event EventBeginPlay
  (bind _outactors (Actor|GetAllActorsOfClass "/Game/Interactables/MagneticFields/BP_NewMagneticFieldCylinder.BP_NewMagneticFieldCylinder_C"))
  (if (> (Utilities|Array|Length _outactors) 0)
    (Variables|Default|SetMagnetic%20Field%20Cylinder (Utilities|Array|Get(acopy) _outactors))))

(event EventTick
  (params (DeltaSeconds :type Float%20%28single-precision%29)))

(event Collision|EventActorBeginOverlap
  (params (OtherActor :type Actor%20Object%20Reference)))

(fn ConstructionScript)