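; Robot character Blueprint that supplies FMOD audio and dash effects for movement, launch and polarity switching.
; BeginPlay binds a movement-state event that toggles a walking audio component and plays one-shot jump and landing sounds.
; Launch and polarity events play, add or stop FMOD components.
; The movement component's dash event spawns a Niagara system attached to the mesh and adds an FMOD component.
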(event OnDashEvent(CharacterMovement)
  (params (IsDashing :type Boolean))
  (Niagara|SpawnSystemAttached "/Game/ParticleSystems/CharacterSystems/NS_Dash2test.NS_Dash2test" (Variables|Character|GetMesh) "None" "0, 0, 0" "0, 0, 0" "SnapToTarget" false)
  (AddComponent|AddFMODAudioComponent false))

(event Custom|OnMovementStateChanged_Event_0
  (params (NewState :type ERobotMovementState%20Enum :default "Idle"))
  (switch Utilities|FlowControl|Switch|SwitchonERobotMovementState NewState
    (:Idle
      (Class|FMODAudioComponent|Stop (Variables|Default|GetWalkingAudioComp)))
    (:Walking
      (Class|FMODAudioComponent|Play (Variables|Default|GetWalkingAudioComp)))
    (:Jumping
      (Class|FMODBlueprintStatics|PlayEventatLocation "/Game/FMOD/Events/PLAYER/Robot_Jump.Robot_Jump" (Math|Conversions|ToTransform(Vector) (Transformation|GetActorLocation))))
    (:Landing
      (Class|FMODBlueprintStatics|PlayEventatLocation "/Game/FMOD/Events/PLAYER/Robot_Land.Robot_Land" (Math|Conversions|ToTransform(Vector) (Transformation|GetActorLocation))))))

(event EventOnSwitchPolarity
  (params (NewPolarity :type EPolarity%20Enum :default "Positive"))
  (switch Utilities|FlowControl|Switch|SwitchonEPolarity NewPolarity
    (:Positive
      (Class|FMODAudioComponent|Play (Variables|Default|GetPolaritySwitchAudioComp)))
    (:Negative
      (AddComponent|AddFMODAudioComponent false))))

(event Collision|EventActorBeginOverlap
  (params (OtherActor :type Actor%20Object%20Reference)))

(event EventTick
  (params (DeltaSeconds :type Float%20%28single-precision%29)))

(event EventOnLaunchEnd
  (AddComponent|AddFMODAudioComponent false)
  (Class|FMODAudioComponent|Stop (stale EventOnLaunchStart _returnvalue)))

(event EventBeginPlay
  (EventDispatchers|AssignOnMovementStateChanged (delegate Custom|OnMovementStateChanged_Event_0)))

(event EventOnLaunchStart
  (bind _returnvalue (AddComponent|AddFMODAudioComponent false)))

(fn ConstructionScript)