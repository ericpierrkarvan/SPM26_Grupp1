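; Spline-driven cable actor that builds a VFX cable mesh with an animated pulse material.
; The construction script splits CableSpline by SegmentLength and adds a Y-forward spline mesh per segment, matching positions and tangents from the spline.
; On BeginPlay, the TL_Pulse timeline writes PulsePosition to the MPC_Cable parameter collection, so the value is global rather than per cable.
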(event EventBeginPlay
  (bind _pulse (Timeline|TL_Pulse Play)
    (:Update
      (Rendering|Material|SetScalarParameterValue "/Game/ParticleSystems/ParticleSystemsBlueprints/MPC_Cable.MPC_Cable" "PulsePosition" _pulse :!class /Script/Engine.KismetMaterialLibrary))))

(event Collision|EventActorBeginOverlap
  (params (OtherActor :type Actor%20Object%20Reference)))

(event EventTick
  (params (DeltaSeconds :type Float%20%28single-precision%29)))

(fn ConstructionScript
  (for _index (range 0 (- (Math|Float|Ceil (/ (Spline|GetSplineLength (Variables|Default|GetCableSpline)) (Variables|Default|GetSegmentLength))) 1))
    (bind _returnvalue (AddComponent|AddSplineMeshComponent false))
    (SplineMesh|SetForwardAxis _returnvalue "Y" true)
    (Components|StaticMesh|SetStaticMesh _returnvalue "/Game/ParticleSystems/ParticleSystemsMeshes/SM_VFXCableSegment100cmx8radius2.SM_VFXCableSegment100cmx8radius2")
    (Rendering|Material|SetMaterial _returnvalue 0 "/Game/ParticleSystems/ParticleSystemsMaterials/M_CablePulse_VFX.M_CablePulse_VFX")
    (SplineMesh|SetStartandEnd _returnvalue (Spline|GetLocationatDistanceAlongSpline (Variables|Default|GetCableSpline) (* _index (Variables|Default|GetSegmentLength)) "Local") (Spline|GetTangentatDistanceAlongSpline (Variables|Default|GetCableSpline) (* _index (Variables|Default|GetSegmentLength)) "Local") (Spline|GetLocationatDistanceAlongSpline (Variables|Default|GetCableSpline) (+ (* _index (Variables|Default|GetSegmentLength)) (Variables|Default|GetSegmentLength)) "Local") (Spline|GetTangentatDistanceAlongSpline (Variables|Default|GetCableSpline) (+ (* _index (Variables|Default|GetSegmentLength)) (Variables|Default|GetSegmentLength)) "Local") true :!class /Script/Engine.SplineMeshComponent)))