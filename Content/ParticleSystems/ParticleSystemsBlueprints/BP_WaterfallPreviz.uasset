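; BP_WaterfallPreviz is an editor previsualization actor that sketches a waterfall's ballistic arc with debug drawing.
; Its construction script flushes persistent debug lines, then draws the segmented path, a marker at a chosen debug time, the apex, and an end ellipse with axes.
; Helper functions compute local positions and apex time from speed, vertical speed and gravity, which the actor transform places in the world.
; The event graph and DrawDebugPath functions are empty.
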(event EventBeginPlay)

(event Collision|EventActorBeginOverlap
  (params (OtherActor :type Actor%20Object%20Reference)))

(event EventTick
  (params (DeltaSeconds :type Float%20%28single-precision%29)))

(fn ConstructionScript
  (bind _returnvalue (Transformation|GetActorTransform))
  (bind _duration (Variables|Default|GetDuration))
  (bind _debugsegments (Variables|Default|GetDebugSegments))
  (bind _returnvalue_2 (Class|KismetMathLibrary|ToInt64(Integer) _debugsegments))
  (Rendering|Debug|FlushPersistentDebugLines)
  ;[0.15 0.15 0.15 0.5] Path
  (for _index (range 0 (- (Variables|Default|GetDebugSegments) 1))
    (Rendering|Debug|DrawDebugLine (Math|Transform|TransformLocation _returnvalue (CallFunction|GetBallisticLocalPos (* (/ (Math|Conversions|ToByte(Integer) _index) _returnvalue_2) _duration))) (Math|Transform|TransformLocation _returnvalue (CallFunction|GetBallisticLocalPos (* _duration (/ (Math|Conversions|ToByte(Integer) (+ _index 1)) _returnvalue_2)))) "(R=1.000000,G=1.000000,B=1.000000,A=1.000000)" 1e+02 1.0))
  ;[0.15 0.15 0.15 0.5] Time
  (Rendering|Debug|DrawDebugPoint (Math|Transform|TransformLocation (Transformation|GetActorTransform) (CallFunction|GetBallisticLocalPos (Variables|Default|GetDebugTime))) 12.0 "(R=1.000000,G=1.000000,B=1.000000,A=1.000000)" 1e+03)
  ;[0.15 0.15 0.15 0.5] Apex
  (Rendering|Debug|DrawDebugPoint (Math|Transform|TransformLocation (Transformation|GetActorTransform) (.Pos (CallFunction|GetBallisticApexLocalPos))) 8.0 "(R=1.000000,G=0.000000,B=0.008427,A=1.000000)" 1e+03)
  ;[0.15 0.15 0.15 0.5] End
  (Rendering|Debug|DrawDebugCircle (Math|Transform|TransformLocation (Transformation|GetActorTransform) (CallFunction|GetBallisticLocalPos (Variables|Default|GetDuration))) 0.5 64 "(R=1.000000,G=1.000000,B=1.000000,A=1.000000)" 1e+03 1.0 (* (Transformation|GetActorRightVector) 1.5e+02) (* (Transformation|GetActorForwardVector) 1e+02) true))

(fn GetBallisticLocalPos
  (params (Time :type Float%20%28double-precision%29))
  (return (+ (* (Math|Vector|MakeVector (Variables|Default|GetSpeed) 0.0 (Variables|Default|GetVerticalSpeed)) Time) (* (* Time Time (Variables|Default|GetGravity) 0.5) "0.000000,0.000000,1.000000"))))

(fn GetBallisticApexLocalPos
  (bind _apextime (CallFunction|GetBallisticApexTime))
  (return (CallFunction|GetBallisticLocalPos _apextime) _apextime))

(fn GetBallisticApexTime
  (return (/ (Variables|Default|GetVerticalSpeed) (Math|Float|Absolute(Float) (Variables|Default|GetGravity)))))

(fn DrawDebugPath)

(fn DrawDebugPathEnd)