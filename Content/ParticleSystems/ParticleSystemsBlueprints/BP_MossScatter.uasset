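; BP_MossScatter is an actor that scatters moss instances over surfaces around its BaseMesh.
; Downward Visibility traces from random points near the mesh's bounds origin place MossInstances at each hit, aligned to the normal with random yaw and scale.
; The construction script builds this using a hardcoded footprint.
; BeginPlay clears and re-scatters using the mesh's local bounds, so the runtime layout differs from the editor's.
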(event EventBeginPlay
  (bind _returnvalue (Math|Random|RandomFloatinRange -0.5 0.5))
  (bind _returnvalue_2 (Math|Random|RandomFloatinRange -0.5 0.5))
  (bind _basemesh (Variables|Default|GetBaseMesh))
  (bind _basemesh_2 (Variables|Default|GetBaseMesh))
  (bind _minscale (Variables|Default|GetMinScale))
  (bind _maxscale (Variables|Default|GetMaxScale))
  (bind _returnvalue_3 (Math|Random|RandomFloatinRange _minscale _maxscale))
  (bind _origin (Collision|GetComponentBounds _basemesh))
  (bind (_min _max) (Components|StaticMesh|GetLocalBounds _basemesh_2))
  (bind _returnvalue_4 (- _max _min))
  (bind (_x _y) (Math|Vector|BreakVector _returnvalue_4))
  (bind _returnvalue_5 (* _y _returnvalue_2))
  (bind _returnvalue_6 (* _x _returnvalue))
  (bind _returnvalue_7 (Math|Vector|MakeVector _returnvalue_6 _returnvalue_5 5e+01))
  (bind _returnvalue_8 (+ _origin _returnvalue_7))
  (Components|InstancedStaticMesh|ClearInstances (Variables|Default|GetMossInstances))
  (for _index (range 0 (Variables|Default|GetScatterCount))
    (bind (_outhit _returnvalue_9) (Collision|LineTraceByChannel _returnvalue_8 (- _returnvalue_8 (Math|Vector|MakeVector 0.0 0.0 (Variables|Default|GetTraceDistance))) "TraceTypeQuery1" false 0 "None"))
    (if _returnvalue_9
      (Components|InstancedStaticMesh|AddInstance (Variables|Default|GetMossInstances) (Math|Transform|MakeTransform (.ImpactPoint (Collision|BreakHitResult _outhit)) (Math|Rotator|MakeRotator (.Roll (Math|Rotator|BreakRotator (Math|Rotator|MakeRotfromZ (.ImpactNormal (Collision|BreakHitResult _outhit))))) (.Pitch (Math|Rotator|BreakRotator (Math|Rotator|MakeRotfromZ (.ImpactNormal (Collision|BreakHitResult _outhit))))) (Math|Random|RandomFloatinRange 0.0 3.6e+02)) (Math|Vector|MakeVector _returnvalue_3 _returnvalue_3 _returnvalue_3)) true))))

(event Collision|EventActorBeginOverlap
  (params (OtherActor :type Actor%20Object%20Reference)))

(event EventTick
  (params (DeltaSeconds :type Float%20%28single-precision%29)))

(fn ConstructionScript
  (bind _returnvalue (Math|Random|RandomFloatinRange -0.5 0.5))
  (bind _returnvalue_2 (Math|Vector|MakeVector 223.0 208.0 189.0))
  (bind _returnvalue_3 (Math|Random|RandomFloatinRange -0.5 0.5))
  (bind _basemesh (Variables|Default|GetBaseMesh))
  (bind _minscale (Variables|Default|GetMinScale))
  (bind _maxscale (Variables|Default|GetMaxScale))
  (bind _returnvalue_4 (Math|Random|RandomFloatinRange _minscale _maxscale))
  (bind _origin (Collision|GetComponentBounds _basemesh))
  (bind (_x _y) (Math|Vector|BreakVector _returnvalue_2))
  (bind _returnvalue_5 (* _y _returnvalue_3))
  (bind _returnvalue_6 (* _x _returnvalue))
  (bind _returnvalue_7 (Math|Vector|MakeVector _returnvalue_6 _returnvalue_5 5e+01))
  (bind _returnvalue_8 (+ _origin _returnvalue_7))
  (Components|InstancedStaticMesh|ClearInstances (Variables|Default|GetMossInstances))
  (for _index (range 0 (Variables|Default|GetScatterCount))
    (bind (_outhit _returnvalue_9) (Collision|LineTraceByChannel _returnvalue_8 (- _returnvalue_8 (Math|Vector|MakeVector 0.0 0.0 (Variables|Default|GetTraceDistance))) "TraceTypeQuery1" false 0 "None"))
    (if _returnvalue_9
      (Components|InstancedStaticMesh|AddInstance (Variables|Default|GetMossInstances) (Math|Transform|MakeTransform (.ImpactPoint (Collision|BreakHitResult _outhit)) (Math|Rotator|MakeRotator (.Roll (Math|Rotator|BreakRotator (Math|Rotator|MakeRotfromZ (.ImpactNormal (Collision|BreakHitResult _outhit))))) (.Pitch (Math|Rotator|BreakRotator (Math|Rotator|MakeRotfromZ (.ImpactNormal (Collision|BreakHitResult _outhit))))) (Math|Random|RandomFloatinRange 0.0 3.6e+02)) (Math|Vector|MakeVector _returnvalue_4 _returnvalue_4 _returnvalue_4)) true))))