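; Magnetic field cylinder actor that handles audio feedback for actors pulled or repelled by its field.
; Magnetic force events tell the affected actor's MagneticComponent to play pull or repel sounds, or to stop them when the force ends.
; EndPlay silences every valid actor still in ActorsInField.
; BeginPlay also adds an FMOD audio component and sets an auto-destroy-when-finished flag.
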(event EventBeginPlay
  (AddComponent|AddFMODAudioComponent false)
  (Variables|Default|SetbAutoDestroyWhenFinished true))

(event Collision|EventActorBeginOverlap
  (params (OtherActor :type Actor%20Object%20Reference)))

(event EventTick
  (params (DeltaSeconds :type Float%20%28single-precision%29)))

(event EventOnMagneticForceEndBP
  (params (Actor :type Actor%20Object%20Reference))
  (if (Utilities|IsValid Actor)
    (Class|MagneticComponent|StopMagneticSounds (Actor|GetComponentbyClass Actor "/Script/SPM26_Grupp1.MagneticComponent"))))

(event EventOnMagneticRepulsionBP
  (params (Actor :type Actor%20Object%20Reference))
  ;[0.15 0.15 0.15 0.5] Play Repel Sound
  (if (Utilities|IsValid Actor)
    (Class|MagneticComponent|PlayRepelSound (Actor|GetComponentbyClass Actor "/Script/SPM26_Grupp1.MagneticComponent"))))

(event EventEndPlay
  (params (EndPlayReason :type EEndPlayReason%20Enum :default "Destroyed"))
  (for _array_element (Variables|Default|GetActorsInField)
    (if (Utilities|IsValid _array_element)
      (Class|MagneticComponent|StopMagneticSounds (Actor|GetComponentbyClass _array_element "/Script/SPM26_Grupp1.MagneticComponent")))))

(event EventOnMagneticPullBP
  (params (Actor :type Actor%20Object%20Reference))
  ;[0.15 0.15 0.15 0.5] Play Pull Sound
  (if (Utilities|IsValid Actor)
    (Class|MagneticComponent|PlayPullSound (Actor|GetComponentbyClass Actor "/Script/SPM26_Grupp1.MagneticComponent"))))

(fn ConstructionScript)